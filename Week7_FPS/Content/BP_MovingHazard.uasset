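; BP_MovingHazard is a hazard that travels back and forth between its start position and a TargetLocation actor, damaging the player while overlapping.
; A timeline lerps the location using the linear, curve or linear-with-wait track chosen by LerpTrack, with Speed as play rate.
; A FlipFlop reverses or replays the timeline on each finish.
; Overlap events cache the player and toggle damage, which Tick applies every frame.
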(event EventBeginPlay
  (if (Utilities|IsValid (Variables|Default|GettargetLocation))
    (Variables|Default|SetstartLocation (Transformation|GetActorLocation))
    (bind (_direction _track_linear _track_curve _track_linearwait) (Timeline|TL_MovingObject Play)
      (:Update
        (switch string (Variables|Default|GetlerpTrack)
          (:Default
            (CallFunction|LerpMoveBackandForth _track_curve :!label _label))
          (:Linear
            (CallFunction|LerpMoveBackandForth _track_linear))
          (:Curve
            (goto _label))
          (:Linear%20Wait
            (CallFunction|LerpMoveBackandForth _track_linearwait))))
      (:Finished
        (Utilities|FlowControl|FlipFlop
          (:A
            (Timeline|TL_MovingObject ReverseFromEnd))
          (:B
            (Timeline|TL_MovingObject PlayFromStart)))))))

(event Collision|EventActorBeginOverlap
  (params (OtherActor :type Actor%20Object%20Reference))
  (bind _asbp_player_character (Utilities|Casting|CastToBP_PlayerCharacter OtherActor))
  (Variables|Default|SetisDamaging true))

(event Collision|EventActorEndOverlap
  (params (OtherActor :type Actor%20Object%20Reference))
  (Utilities|Casting|CastToBP_PlayerCharacter OtherActor)
  (Variables|Default|SetisDamaging false))

(event EventTick
  (params (DeltaSeconds :type Float%20%28single-precision%29))
  (if (Variables|Default|GetisDamaging)
    (Default|TakeDamage (stale Collision|EventActorBeginOverlap _asbp_player_character) (Variables|Default|GetdamageAmount) "/Game/sfx_playerDamaged.sfx_playerDamaged")))

(fn ConstructionScript)

(fn LerpMoveBackandForth
  (params (Lerp%20Alpha :type Float%20%28double-precision%29))
  (Components|Timeline|SetPlayRate (Variables|Default|GetTL_MovingObject) (Variables|Default|Getspeed))
  (Transformation|SetActorLocation (Math|Vector|Lerp(Vector) (Variables|Default|GetstartLocation) (Transformation|GetActorLocation (Variables|Default|GettargetLocation)) Lerp%20Alpha) false false))