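; BP_ShootingObject is a shootable enemy that fires BP_EnemyBullet at the player while PlayerInRadius is set, rate-limited by a delay.
; A FlipFlopped timeline ping-pongs it between its start and a TargetLocation actor, using a selectable track and speed.
; Tick turns it toward the player and tints its sphere green while the player is in radius.
; Only then does a BP_Bullet overlap award a point and destroy it with its ViewRadius.
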(event EventBeginPlay
  (if (Utilities|IsValid (Variables|Default|GettargetLocation))
    (Variables|Default|SetstartLocation (Transformation|GetActorLocation))
    (bind (_direction _track_linear _track_curve _track_linearwait) (Timeline|TL_MovingObject Play)
      (:Update
        (switch string (Variables|Default|GetlerpTrack)
          (:Default
            (CallFunction|LerpMoveBackandForth _track_curve :!label _label))
          (:Linear
            (CallFunction|LerpMoveBackandForth _track_linear))
          (:Curve
            (goto _label))
          (:Linear%20Wait
            (CallFunction|LerpMoveBackandForth _track_linearwait))))
      (:Finished
        (Utilities|FlowControl|FlipFlop
          (:A
            (Timeline|TL_MovingObject ReverseFromEnd))
          (:B
            (Timeline|TL_MovingObject PlayFromStart)))))))

(event Collision|EventActorBeginOverlap
  (params (OtherActor :type Actor%20Object%20Reference))
  ;[1 1 1] On hit
  (Utilities|Casting|CastToBP_Bullet OtherActor)
  (if (Variables|Default|GetplayerInRadius)
    (bind _outactors (Actor|GetAllActorsOfClass "/Game/BP_PlayerCharacter.BP_PlayerCharacter_C"))
    (Math|Integer|IncrementInt (Variables|/Game/BP_PlayerCharacter.BP_PlayerCharacter_C|Getpoints (Utilities|Array|Get(acopy) _outactors))
      (:%20%20
        (Audio|PlaySoundatLocation "/Engine/VREditor/Sounds/UI/Camera_Shutter.Camera_Shutter" (Transformation|GetActorLocation) "0, 0, 0" 1.0 1.0 0.0 0 0 0 0)
        (Actor|DestroyActor (Variables|Default|GetviewRadius))
        (Actor|DestroyActor)))))

(event EventTick
  (params (DeltaSeconds :type Float%20%28single-precision%29))
  (CallFunction|UpdateSphereMaterial)
  (CallFunction|TurnTowardsPlayer)
  ;[1 1 1] Shoot at player
  (if (and (Variables|Default|GetplayerInRadius) (not (Variables|Default|GetisBuffering)))
    (Game|SpawnActorfromClass "/Game/BP_EnemyBullet.BP_EnemyBullet_C" (Transformation|GetActorTransform) "Undefined" "MultiplyWithRoot" 0 0)
    (Variables|Default|SetisBuffering true)
    (Utilities|FlowControl|Delay (Variables|Default|GetshootBuffer))
    (Variables|Default|SetisBuffering false)))

(fn ConstructionScript)

(fn LerpMoveBackandForth
  (params (Lerp%20Alpha :type Float%20%28double-precision%29))
  (Components|Timeline|SetPlayRate (Variables|Default|GetTL_MovingObject) (Variables|Default|Getspeed))
  (Transformation|SetActorLocation (Math|Vector|Lerp(Vector) (Variables|Default|GetstartLocation) (Transformation|GetActorLocation (Variables|Default|GettargetLocation)) Lerp%20Alpha) false false))

(fn TurnTowardsPlayer
  (bind _outactors (Actor|GetAllActorsOfClass "/Game/BP_PlayerCharacter.BP_PlayerCharacter_C"))
  (Transformation|SetActorRotation (Math|Rotator|FindLookatRotation (Transformation|GetActorLocation) (Transformation|GetActorLocation (Utilities|Array|Get(acopy) _outactors)))))

(fn UpdateSphereMaterial
  (if (Variables|Default|GetplayerInRadius)
    (Rendering|Material|SetMaterial (Variables|Default|GetSphere) 0 "/Engine/EngineDebugMaterials/VertexColorViewMode_GreenOnly.VertexColorViewMode_GreenOnly")
    (else
      (Rendering|Material|SetMaterial (Variables|Default|GetSphere) 0 "/Engine/BasicShapes/BasicShapeMaterial.BasicShapeMaterial"))))