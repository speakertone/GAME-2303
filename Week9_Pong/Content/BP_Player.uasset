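; BP_Player is the player Blueprint that slides its Cube along local Z using mouse input.
; Tick applies a swept local offset from an input axis value, scaled by Speed and delta time, with a higher multiplier in mouse wheel mode.
; The Click action selects mouse movement and the Mouse Wheel action selects wheel movement by setting the MouseWheelControl flag.
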(event EventBeginPlay)

(event Collision|EventActorBeginOverlap
  (params (OtherActor :type Actor%20Object%20Reference)))

(event EventTick
  (params (DeltaSeconds :type Float%20%28single-precision%29))
  (bind _cube (Variables|Default|GetCube))
  (bind _speed (Variables|Default|Getspeed))
  (if (Variables|Default|GetmouseWheelControl)
    ;[1 1 1] Move with mousewheel
    (Transformation|AddLocalOffset _cube (Math|Vector|MakeVector 0.0 0.0 (* DeltaSeconds (Class|Actor|GetInputAxisKeyValue) _speed 3.0)) true false)
    (else
      ;[1 1 1] Move with mouse
      (Transformation|AddLocalOffset _cube (Math|Vector|MakeVector 0.0 0.0 (* DeltaSeconds (Class|Actor|GetInputAxisKeyValue) _speed)) true false))))

(event Input|ActionEvents|InputActionClick
  (params (Key :type Key%20Structure :default "None"))
  (:Pressed
    (Variables|Default|SetmouseWheelControl false)))

(event Input|ActionEvents|InputActionMouseWheel
  (params (Key :type Key%20Structure :default "None"))
  (:Pressed
    (Variables|Default|SetmouseWheelControl true)))

(fn ConstructionScript)