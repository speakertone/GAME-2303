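; Invisible companion ball for Pong that launches along the current BP_PongBall's trajectory at a multiplied speed and stops near the enemy paddle.
; Copies speed and direction from the real ball on construction, then sets physics velocity on BeginPlay.
; Each tick clamps its Y position, zeroes velocity near the enemy side, and shows the sphere only if BP_PlayerPaddle's SeeInvisibleBall flag is set.
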(event EventBeginPlay
  (Physics|SetPhysicsLinearVelocity (Variables|Default|GetSphere) (* (Math|Vector|MakeVector 0.0 (Variables|Default|GetdirectionY) (Variables|Default|GetdirectionZ)) (Variables|Default|Getspeed) (Variables|Default|GetspeedMultiplier)) false "None"))

(event EventTick
  (params (DeltaSeconds :type Float%20%28single-precision%29))
  (bind _sphere (Variables|Default|GetSphere))
  (bind _returnvalue (Transformation|GetWorldLocation _sphere))
  (CallFunction|UpdateVisibility)
  (Transformation|SetWorldLocation _sphere (Math|Vector|MakeVector 0.0 (Math|Float|Clamp(Float) (.y _returnvalue) -2e+03 1.45e+03) (.z _returnvalue)) false false)
  ;[1 1 1] Freeze in place if close enough to enemy paddle
  (if (>= (.y _returnvalue) 1.4e+03)
    (Physics|SetPhysicsLinearVelocity _sphere "0, 0, 0" false "None")))

(fn ConstructionScript
  (bind _returnvalue (Actor|GetActorOfClass "/Game/BP_PongBall.BP_PongBall_C"))
  (if (Utilities|IsValid _returnvalue)
    (Variables|Default|Setspeed (Variables|/Game/BP_PongBall.BP_PongBall_C|Getspeed _returnvalue))
    (Variables|Default|SetdirectionY (Variables|/Game/BP_PongBall.BP_PongBall_C|GetdirectionY _returnvalue))
    (Variables|Default|SetdirectionZ (Variables|/Game/BP_PongBall.BP_PongBall_C|GetdirectionZ _returnvalue))))

(fn UpdateVisibility
  (bind _returnvalue (Actor|GetActorOfClass "/Game/BP_PlayerPaddle.BP_PlayerPaddle_C"))
  (Rendering|SetVisibility (Variables|Default|GetSphere) (Variables|/Game/BP_PlayerPaddle.BP_PlayerPaddle_C|GetseeInvisibleBall _returnvalue) false))