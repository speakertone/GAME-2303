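; Pong ball actor that moves by physics velocity and scores for the player or enemy paddle on passing either Y-axis limit.
; Paddle hits increase its speed and set a new Y/Z direction from the hit point relative to the paddle.
; Player hits spawn a BP_InvisibleBall at its location, cleared on the next paddle hit or score.
; After a score, it asks BP_BallSpawner for a new ball and destroys itself.
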(event EventBeginPlay
  (Physics|SetPhysicsLinearVelocity (Variables|Default|GetSphere) (Math|Vector|MakeVector 0.0 (* (Variables|Default|Getspeed) -1.0) 0.0) false "None"))

(event EventTick
  (params (DeltaSeconds :type Float%20%28single-precision%29))
  (bind _sphere (Variables|Default|GetSphere))
  (bind _returnvalue (Transformation|GetWorldLocation _sphere))
  (if (>= (.y _returnvalue) 2e+03)
    ;[1 1 1] Player gets a point
    (bind _returnvalue_2 (Actor|GetActorOfClass "/Game/BP_PlayerPaddle.BP_PlayerPaddle_C"))
    (Math|Integer|IncrementInt (Variables|/Game/BP_Paddle.BP_Paddle_C|Getscore _returnvalue_2)
      (:%20%20
        (bind _returnvalue_3 (Actor|GetActorOfClass "/Game/BP_BallSpawner.BP_BallSpawner_C" :!label _label))
        (Default|SpawnBall _returnvalue_3)
        (CallFunction|DestroyInvisibleBall)
        (Actor|DestroyActor)))
    (elif (<= (.y _returnvalue) -2e+03)
      ;[1 1 1] Computer gets a point
      (bind _returnvalue_4 (Actor|GetActorOfClass "/Game/BP_EnemyPaddle.BP_EnemyPaddle_C"))
      (Math|Integer|IncrementInt (Variables|/Game/BP_Paddle.BP_Paddle_C|Getscore _returnvalue_4)
        (:%20%20
          (goto _label))))))

(event Collision|EventHit
  (params (MyComp :type Primitive%20Component%20Object%20Reference) (Other :type Actor%20Object%20Reference) (OtherComp :type Primitive%20Component%20Object%20Reference) (bSelfMoved :type Boolean) (HitLocation :type Vector :default "0, 0, 0") (HitNormal :type Vector :default "0, 0, 0") (NormalImpulse :type Vector :default "0, 0, 0") (Hit :type Hit%20Result%20Structure%20%28by%20ref%29))
  (bind _asbp_paddle (Utilities|Casting|CastToBP_Paddle Other))
  (CallFunction|DestroyInvisibleBall)
  ;[1 1 1] Increase ball speed on each hit
  (Variables|Default|Setspeed (+ (Variables|Default|Getspeed) (Variables|Default|GetspeedIncrement)))
  ;[1 1 1] Set direction
  (if (>= (.y HitLocation) (.y (Transformation|GetWorldLocation (Variables|/Game/BP_Paddle.BP_Paddle_C|GetCube _asbp_paddle))))
    (Variables|Default|SetdirectionY 1.0)
    (else
      (Variables|Default|SetdirectionY -1.0)))
  (Variables|Default|SetdirectionZ (Math|Float|NormalizetoRange (- (.z HitLocation) (.z (Transformation|GetWorldLocation (Variables|/Game/BP_Paddle.BP_Paddle_C|GetCube _asbp_paddle)))) 0.0 8e+01))
  (Physics|SetPhysicsLinearVelocity (Variables|Default|GetSphere) (* (Math|Vector|MakeVector 0.0 (Variables|Default|GetdirectionY) (Variables|Default|GetdirectionZ)) (Variables|Default|Getspeed)) false "None")
  ;[1 1 1] Spawn invisible ball
  (Utilities|Casting|CastToBP_PlayerPaddle Other)
  (Game|SpawnActorfromClass "/Game/BP_InvisibleBall.BP_InvisibleBall_C" (Math|Transform|MakeTransform (Transformation|GetActorLocation) "0, 0, 0" "1.000000,1.000000,1.000000") "Undefined" "MultiplyWithRoot" 0 0))

(fn ConstructionScript)

(fn DestroyInvisibleBall
  (bind _returnvalue (Actor|GetActorOfClass "/Game/BP_InvisibleBall.BP_InvisibleBall_C"))
  (if (Utilities|IsValid _returnvalue)
    (Actor|DestroyActor _returnvalue)))