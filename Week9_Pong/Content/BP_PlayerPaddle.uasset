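; BP_PlayerPaddle is the player-controlled paddle, which also adds the BP_HUD widget to the viewport at BeginPlay.
; Each tick it moves its Cube along local Z with sweep, scaled by axis input, Speed and delta time, with a higher multiplier for mouse-wheel control.
; Click and Mouse Wheel actions switch between mouse and wheel control, while ToggleInvisibility flips the SeeInvisibleBall flag through a FlipFlop.
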(event EventBeginPlay
  (|CallParentFunction)
  (bind _returnvalue (UserInterface|CreateWidget "/Game/BP_HUD.BP_HUD_C"))
  (UserInterface|Viewport|AddtoViewport _returnvalue 0))

(event Collision|EventActorBeginOverlap
  (params (OtherActor :type Actor%20Object%20Reference))
  (|CallParentFunction OtherActor) ; This node is disabled and will not be called.\nDrag off pins to build functionality.
)

(event EventTick
  (params (DeltaSeconds :type Float%20%28single-precision%29))
  (bind _speed (Variables|Default|Getspeed))
  (bind _cube (Variables|Default|GetCube))
  (|CallParentFunction DeltaSeconds)
  (if (Variables|Default|GetmouseWheelControl)
    ;[1 1 1] Move with mousewheel
    (Transformation|AddLocalOffset _cube (Math|Vector|MakeVector 0.0 0.0 (* DeltaSeconds (Class|Actor|GetInputAxisKeyValue) _speed 3.0)) true false)
    (else
      ;[1 1 1] Move with mouse
      (Transformation|AddLocalOffset _cube (Math|Vector|MakeVector 0.0 0.0 (* DeltaSeconds (Class|Actor|GetInputAxisKeyValue) _speed)) true false))))

(event Input|ActionEvents|InputActionClick
  (params (Key :type Key%20Structure :default "None"))
  (:Pressed
    (Variables|Default|SetmouseWheelControl false)))

(event Input|ActionEvents|InputActionMouseWheel
  (params (Key :type Key%20Structure :default "None"))
  (:Pressed
    (Variables|Default|SetmouseWheelControl true)))

(event Input|ActionEvents|InputActionToggleInvisibility
  (params (Key :type Key%20Structure :default "None"))
  (:Pressed
    (bind _isa (Utilities|FlowControl|FlipFlop)
      (:A
        _)
      (:B
        _))
    (Variables|Default|SetseeInvisibleBall _isa)))

(fn ConstructionScript
  (|CallParentFunction))