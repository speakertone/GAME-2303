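; BP_EnemyPaddle is an AI-controlled paddle that tracks the invisible ball along the vertical axis.
; Each Tick it looks up the BP_InvisibleBall actor and, if valid, clamps that ball's world Z to fixed bounds.
; It then moves its Cube component toward that height with MoveComponentTo over MoveTime, which sets how quickly the paddle reacts.
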(event EventBeginPlay
  (|CallParentFunction) ; This node is disabled and will not be called.\nDrag off pins to build functionality.
)

(event Collision|EventActorBeginOverlap
  (params (OtherActor :type Actor%20Object%20Reference))
  (|CallParentFunction OtherActor) ; This node is disabled and will not be called.\nDrag off pins to build functionality.
)

(event EventTick
  (params (DeltaSeconds :type Float%20%28single-precision%29))
  (|CallParentFunction DeltaSeconds)
  (bind _returnvalue (Actor|GetActorOfClass "/Game/BP_InvisibleBall.BP_InvisibleBall_C"))
  (if (Utilities|IsValid _returnvalue)
    (Components|MoveComponentTo (Variables|Default|GetCube) (Math|Vector|MakeVector 0.0 0.0 (Math|Float|Clamp(Float) (.z (Transformation|GetActorLocation _returnvalue)) -875.0 875.0)) "0, 0, 0" false false (Variables|Default|GetmoveTime) false)))

(fn ConstructionScript
  (|CallParentFunction))